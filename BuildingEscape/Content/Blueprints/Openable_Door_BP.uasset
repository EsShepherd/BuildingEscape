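; Openable door actor that swings open and closed in response to events from its OpenDoor component.
; BeginPlay stores the starting rotation, and the DoorSwing timeline lerps yaw from zero to the component's open angle, combined with that rotation.
; Closing reverses the same timeline, and each direction plays the component's open or close sound at the door's location.
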(event OnOpen(OpenDoor)
  ;[1 1 1] Open Door
  (Audio|PlaySoundatLocation (Variables|/Script/BuildingEscape.OpenDoor|GetOpenSound (Variables|Default|GetOpenDoor)) (Transformation|GetActorLocation) "0, 0, 0" 1.0 1.0 0.0 0 0 0)
  (bind _open_angle (Timeline|DoorSwing Play)
    (:Update
      (Transformation|SetActorRotation (Math|Rotator|CombineRotators (Math|Rotator|MakeRotator 0.0 0.0 (Math|Float|Lerp 0.0 (Class|OpenDoor|GetOpenAngle (Variables|Default|GetOpenDoor)) _open_angle)) (Variables|Default|GetInitial%20Angle))))))

(event OnClose(OpenDoor)
  ;[1 1 1] Open Door
  (Audio|PlaySoundatLocation (Variables|/Script/BuildingEscape.OpenDoor|GetCloseSound (Variables|Default|GetOpenDoor)) (Transformation|GetActorLocation) "0, 0, 0" 1.0 1.0 0.0 0 0 0)
  (bind _open_angle (Timeline|DoorSwing Reverse)
    (:Update
      (Transformation|SetActorRotation (Math|Rotator|CombineRotators (Math|Rotator|MakeRotator 0.0 0.0 (Math|Float|Lerp 0.0 (Class|OpenDoor|GetOpenAngle (Variables|Default|GetOpenDoor)) _open_angle)) (Variables|Default|GetInitial%20Angle))))))

(event Collision|EventActorBeginOverlap
  (params (OtherActor :type Actor%20Object%20Reference)))

(event EventTick
  (params (DeltaSeconds :type Float%20%28single-precision%29)))

(event EventBeginPlay
  ;[1 1 1] Open Door
  (Variables|Default|SetInitial%20Angle (Transformation|GetActorRotation)))

(fn ConstructionScript
  (|CallParentFunction))

(fn NewFunction0)